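; WorldPlaceableText is a Blueprint that displays up to ten lines of text through a widget component, apparently as placeable text in the world.
; On BeginPlay it creates a SimpleText widget, assigns it to the Widget component and copies each Line variable into its matching text block.
; The construction script is empty and nothing updates afterwards, so the text is set once at runtime.
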(event EventBeginPlay
  (bind _returnvalue (UserInterface|CreateWidget "/Game/Widgets/SimpleText.SimpleText_C"))
  (UserInterface|SetWidget (Variables|Default|GetWidget) _returnvalue)
  (Rendering|Components|TextRender|SetText (Variables|/Game/Widgets/SimpleText.SimpleText_C|GetTextBlock1 _returnvalue) (Utilities|Text|ToText(String) (Variables|Default|GetLine1)))
  (Rendering|Components|TextRender|SetText (Variables|/Game/Widgets/SimpleText.SimpleText_C|GetTextBlock2 _returnvalue) (Utilities|Text|ToText(String) (Variables|Default|GetLine2)))
  (Rendering|Components|TextRender|SetText (Variables|/Game/Widgets/SimpleText.SimpleText_C|GetTextBlock3 _returnvalue) (Utilities|Text|ToText(String) (Variables|Default|GetLine3)))
  (Rendering|Components|TextRender|SetText (Variables|/Game/Widgets/SimpleText.SimpleText_C|GetTextBlock4 _returnvalue) (Utilities|Text|ToText(String) (Variables|Default|GetLine4)))
  (Rendering|Components|TextRender|SetText (Variables|/Game/Widgets/SimpleText.SimpleText_C|GetTextBlock5 _returnvalue) (Utilities|Text|ToText(String) (Variables|Default|GetLine5)))
  (Rendering|Components|TextRender|SetText (Variables|/Game/Widgets/SimpleText.SimpleText_C|GetTextBlock6 _returnvalue) (Utilities|Text|ToText(String) (Variables|Default|GetLine6)))
  (Rendering|Components|TextRender|SetText (Variables|/Game/Widgets/SimpleText.SimpleText_C|GetTextBlock7 _returnvalue) (Utilities|Text|ToText(String) (Variables|Default|GetLine7)))
  (Rendering|Components|TextRender|SetText (Variables|/Game/Widgets/SimpleText.SimpleText_C|GetTextBlock8 _returnvalue) (Utilities|Text|ToText(String) (Variables|Default|GetLine8)))
  (Rendering|Components|TextRender|SetText (Variables|/Game/Widgets/SimpleText.SimpleText_C|GetTextBlock9 _returnvalue) (Utilities|Text|ToText(String) (Variables|Default|GetLine9)))
  (Rendering|Components|TextRender|SetText (Variables|/Game/Widgets/SimpleText.SimpleText_C|GetTextBlock10 _returnvalue) (Utilities|Text|ToText(String) (Variables|Default|GetLine10))))

(fn ConstructionScript)