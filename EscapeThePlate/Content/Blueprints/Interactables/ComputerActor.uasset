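; Interactable computer that ingredient characters operate by bumping colliders to enter a PIN, log in and order an Ooba.
; The keyboard overlap cycles the current digit, while the sphere overlap advances to the next and checks all four against the solution.
; A wrong PIN resets the entry and shows an error on the linked ComputerScreen widget.
; Once logged in, the sphere places a one-time order that triggers OobaEscapeZone movement and advances the game mode's task.
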(event OnComponentBeginOverlap(KeyboardCollider)
  (params (OverlappedComponent :type Primitive%20Component%20Object%20Reference) (OtherActor :type Actor%20Object%20Reference) (OtherComp :type Primitive%20Component%20Object%20Reference) (OtherBodyIndex :type Integer) (bFromSweep :type Boolean) (SweepResult :type Hit%20Result%20Structure%20%28by%20ref%29))
  (bind _passwordentered (Variables|Default|GetPasswordEntered))
  (bind _pinidx (Variables|Default|GetPINIdx))
  (Utilities|Casting|CastToIngredientBaseCharacter OtherActor)
  (if (not (Variables|Default|GetLoggedIn))
    (Development|PrintString "Keypress")
    (Utilities|Array|SetArrayElem _passwordentered _pinidx (+ (Utilities|Array|Get(acopy) _passwordentered _pinidx) 1))
    (if (>= (Utilities|Array|Get(acopy) _passwordentered _pinidx) 10)
      (Utilities|Array|SetArrayElem _passwordentered _pinidx 0))))

(event OnComponentBeginOverlap(Sphere)
  (params (OverlappedComponent :type Primitive%20Component%20Object%20Reference) (OtherActor :type Actor%20Object%20Reference) (OtherComp :type Primitive%20Component%20Object%20Reference) (OtherBodyIndex :type Integer) (bFromSweep :type Boolean) (SweepResult :type Hit%20Result%20Structure%20%28by%20ref%29))
  (bind _screen (Variables|Default|GetScreen))
  (bind _passwordentered (Variables|Default|GetPasswordEntered))
  (Utilities|Casting|CastToIngredientBaseCharacter OtherActor)
  (Development|PrintString "KeyClick")
  (if (Variables|Default|GetLoggedIn)
    (if (not (Variables|Default|GetOoobaOrdered))
      (Variables|Default|SetOoobaOrdered true)
      (Default|OobaOrdered (Variables|Default|GetScreen))
      (bind _returnvalue (Actor|GetActorOfClass "/Game/Blueprints/Interactables/OobaEscapeZone.OobaEscapeZone_C"))
      (Default|TriggerMoveto _returnvalue)
      (bind _asbpescape_the_plate_game_mode (Utilities|Casting|CastToBPEscapeThePlateGameMode (Game|GetGameMode)))
      (Class|EscapethePlateGameMode|NextTask _asbpescape_the_plate_game_mode))
    (else
      (bind _output_get (Variables|Default|SetPINIdx (+ (Variables|Default|GetPINIdx) 1)))
      (if (== _output_get 4)
        (Variables|Default|SetPINIdx 0)
        (bind _iscorrect (CallFunction|CheckPassword))
        (if _iscorrect
          (Variables|Default|SetLoggedIn true)
          (Default|Login _screen)
          (Development|PrintString "Logged in")
          (else
            (for (_ _array_index) _passwordentered
              (Utilities|Array|SetArrayElem _passwordentered _array_index 0))
            (Widget|SetVisibility (Variables|/Game/Widgets/ComputerScreen.ComputerScreen_C|GetWrongText _screen) "Visible")
            (Development|PrintString "Bad password")))))))

(event EventBeginPlay
  (bind _ascomputer_screen (Utilities|Casting|CastToComputerScreen (UserInterface|GetUserWidgetObject (Variables|Default|GetWidget))))
  (bind _output_get (Variables|Default|SetScreen _ascomputer_screen))
  (Variables|/Game/Widgets/ComputerScreen.ComputerScreen_C|SetOwningComputer _output_get self))

(fn ConstructionScript)

(fn CheckPassword
  (for (_array_element _array_index) (Variables|Default|GetPasswordEntered)
    (if (!= _array_element (Utilities|Array|Get(acopy) (Variables|Default|GetPasswordSolution) _array_index))
      (return false)))
  (return true))