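; OobaEscapeZone is an interactable actor, named as an escape zone, that slides along the world Y axis when triggered.
; Its TriggerMoveTo event stores the current location as the start point and plays the MoveForward timeline.
; Each timeline update adds the MoveTrack value to the starting Y and sets the location without sweeping.
; The file has no overlap or escape logic.
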(event Custom|TriggerMoveTo
  (Variables|Default|SetStartLocation (Transformation|GetActorLocation))
  (bind _movetrack (Timeline|MoveForward Play)
    (:Update
      (Transformation|SetActorLocation (Math|Vector|MakeVector (.X (Math|Vector|BreakVector (Variables|Default|GetStartLocation))) (+ (.Y (Math|Vector|BreakVector (Variables|Default|GetStartLocation))) _movetrack) (.Z (Math|Vector|BreakVector (Variables|Default|GetStartLocation)))) false false))))

(event EventBeginPlay
  (|CallParentFunction) ; This node is disabled and will not be called.\nDrag off pins to build functionality.
)

(event Collision|EventActorBeginOverlap
  (params (OtherActor :type Actor%20Object%20Reference))
  (|CallParentFunction OtherActor) ; This node is disabled and will not be called.\nDrag off pins to build functionality.
)

(event EventTick
  (params (DeltaSeconds :type Float%20%28single-precision%29))
  (|CallParentFunction DeltaSeconds) ; This node is disabled and will not be called.\nDrag off pins to build functionality.
)

(fn ConstructionScript
  (|CallParentFunction))