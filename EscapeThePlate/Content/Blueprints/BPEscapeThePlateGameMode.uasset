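; Game mode for Escape The Plate that runs a level's ingredient characters, HUD, pause and game-over flow.
; Switching characters refocuses the HUD with a sound and black fade while input is briefly disabled.
; Status changes refresh HUD icons, then either end the game or auto-repossess a character.
; Game over records time and shows win or loss with stars; wins save results through the game instance, and pausing is disabled on the start level.
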(event Custom|SetupHUD
  (bind _returnvalue (UserInterface|CreateWidget "/Game/Widgets/HUDWidget.HUDWidget_C"))
  (bind _output_get (Variables|Default|SetHUD _returnvalue))
  (UserInterface|Viewport|AddtoViewport _output_get 0)
  (Development|PrintString "SetupHUD")
  (Development|PrintString (Utilities|GetDisplayName (Variables|Default|GetHUD)))
  (Default|PopulateCharacterImages (Variables|Default|GetHUD) (Variables|Default|GetCharacters)))

(event EventBeginPlay
  (Class|EscapethePlateGameMode|MakeChaseMusic)
  (Development|PrintString "BEGIN")
  (bind _inplayablemap (CallFunction|IsPlayerinPlayableMap))
  (bind _output_get (Variables|Default|SetbCanPlayerPause _inplayablemap))
  (if _output_get
    (bind _returnvalue (UserInterface|CreateWidget "/Game/Widgets/PauseMenu.PauseMenu_C"))
    (bind _output_get_2 (Variables|Default|SetPauseMenu _returnvalue))
    (Development|PrintString "Menu" true true "(R=0.000000,G=0.660000,B=1.000000,A=1.000000)" 2e+01)
    (Development|PrintString (Utilities|GetDisplayName _output_get_2) true true "(R=0.000000,G=0.660000,B=1.000000,A=1.000000)" 2e+01)
    (else
      (Development|PrintString "Cant pause"))))

(event EventCharacterPossessionChanged
  (bind _returnvalue (Game|GetPlayerController 0))
  (bind _playercameramanager (Variables|/Script/Engine.PlayerController|GetPlayerCameraManager _returnvalue))
  (bind _asingredient_base_character (Utilities|Casting|CastToIngredientBaseCharacter (Pawn|GetControlledPawn _returnvalue)))
  (Default|ChangeCharacterinFocus (Variables|Default|GetHUD) _asingredient_base_character)
  (Audio|PlaySound2D "/Game/Assets/Sound/TransitionSC.TransitionSC" 1.0 1.0 0.0 0 0)
  (Input|DisableInput _returnvalue _returnvalue)
  (CameraFades|StartCameraFade _playercameramanager 1.0 1.0 0.5 "(R=0.000000,G=0.000000,B=0.000000,A=1.000000)" false false)
  (Utilities|FlowControl|Delay 0.5)
  (CameraFades|StartCameraFade _playercameramanager 1.0 0.0 1.0 "(R=0.000000,G=0.000000,B=0.000000,A=1.000000)" false false)
  (Input|EnableInput _returnvalue _returnvalue))

(event EventCharacterStatusChanged
  (for (_array_element _array_index) (Variables|Default|GetCharacters)
    (Default|CharacterStatusIconUpdate (Variables|Default|GetHUD) _array_index _array_element))
  (bind _returnvalue (Class|EscapethePlateGameMode|CheckGameOver))
  (if _returnvalue
    (Development|PrintString "Game Over!")
    (Class|EscapethePlateGameMode|GameOver)
    (else
      (Class|EscapethePlateGameMode|AutoReposessCharacter))))

(event EventGameOver
  (Class|EscapethePlateGameMode|RecordGameTime)
  (bind _returnvalue (UserInterface|CreateWidget "/Game/Widgets/GameOverMenu.GameOverMenu_C"))
  (Input|SetInputModeUIOnly (Game|GetPlayerController 0) _returnvalue "DoNotLock")
  (bind _returnvalue_2 (Class|EscapethePlateGameMode|DidPlayerWin))
  (Class|EscapethePlateGameMode|PlayGameOverMusic _returnvalue_2)
  (if _returnvalue_2
    (Widget|SetVisibility (Variables|/Game/Widgets/GameOverMenu.GameOverMenu_C|GetEscapedLogo _returnvalue) "Visible")
    (else
      (Widget|SetVisibility (Variables|/Game/Widgets/GameOverMenu.GameOverMenu_C|GetTrashedLogo _returnvalue) "Visible")))
  (bind _returnvalue_3 (Class|EscapethePlateGameMode|GetStarsEarned))
  (Default|UpdateStarsEarned _returnvalue _returnvalue_3)
  (UserInterface|Viewport|AddtoViewport _returnvalue 0)
  (Variables|/Script/Engine.PlayerController|SetbShowMouseCursor (Game|GetPlayerController 0) true)
  (Variables|Default|SetbCanPlayerPause false)
  (if _returnvalue_2
    (bind _returnvalue_4 (Class|EscapethePlateGameMode|GetRecordedTime))
    (bind _asbpescape_the_plate_game_instance (Utilities|Casting|CastToBPEscapeThePlateGameInstance (Game|GetGameInstance)))
    (Class|EscapethePlateGameInstance|AddDatatoSave _asbpescape_the_plate_game_instance (Utilities|Struct|MakeLevelSaveData (Variables|Default|GetLevelName) _returnvalue_3 _returnvalue_4 (Variables|Default|GetHasChallengeCompleted)))
    (Class|EscapethePlateGameInstance|SaveGame _asbpescape_the_plate_game_instance)
    (Game|SetGamePaused true)))

(event EventPauseGame
  (bind _returnvalue (Game|GetPlayerController 0))
  (bind _pausemenu (Variables|Default|GetPauseMenu))
  (if (Variables|Default|GetbCanPlayerPause)
    (UserInterface|Viewport|AddtoViewport _pausemenu 0)
    (Input|SetInputModeUIOnly _returnvalue _pausemenu "DoNotLock")
    (Variables|/Script/Engine.PlayerController|SetbShowMouseCursor _returnvalue true)
    (Game|SetGamePaused true)))

(fn ConstructionScript)

(fn IsPlayerinPlayableMap
  (bind _returnvalue (Game|GetCurrentLevelName true))
  (return (Utilities|Enum|NotEqual(Enum) _returnvalue "StartLevel")))