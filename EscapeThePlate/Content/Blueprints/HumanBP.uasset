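; Human AI character that spots usable ingredient characters, grabs and kills them, then carries them until thrown out.
; While empty-handed, AI perception writes sighted usable ingredients to the Blackboard.
; A grab sphere tracks the overlapping ingredient, which AttemptGrab kills and snaps to a hand socket when TryingGrab is set, flagging the Blackboard as holding.
; ThrowOutIngredient detaches it and clears the local holding state, leaving the Blackboard flag untouched.
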(event OnTargetPerceptionUpdated(AIPerception)
  (params (Actor :type Actor%20Object%20Reference) (Stimulus :type AI%20Stimulus%20Structure))
  (bind _returnvalue (AI|GetBlackboard 0))
  ;[1 1 1] Vision detection for ingredient
  (Development|PrintString "sense changed")
  (if (not (Variables|Default|GetHoldingIngredient))
    (bind _asingredient_base_character (Utilities|Casting|CastToIngredientBaseCharacter Actor))
    (bind _returnvalue_2 (Class|IngredientBaseCharacter|IsIngredientUsable _asingredient_base_character))
    (if _returnvalue_2
      (AI|Components|Blackboard|SetValueasBool _returnvalue (Utilities|Name|MakeLiteralName "IngredientSeen") (.bSuccessfullySensed (Utilities|Struct|BreakAIStimulus Stimulus)))
      (AI|Components|Blackboard|SetValueasObject _returnvalue (Utilities|Name|MakeLiteralName "DetectedCharacter") _asingredient_base_character))))

(event OnComponentEndOverlap(GrabSphere)
  (params (OverlappedComponent :type Primitive%20Component%20Object%20Reference) (OtherActor :type Actor%20Object%20Reference) (OtherComp :type Primitive%20Component%20Object%20Reference) (OtherBodyIndex :type Integer))
  ;[1 1 1] Grab and kill players
  (Utilities|Casting|CastToIngredientBaseCharacter OtherActor)
  (Variables|Default|SetIngredientInSphere 0))

(event OnComponentBeginOverlap(GrabSphere)
  (params (OverlappedComponent :type Primitive%20Component%20Object%20Reference) (OtherActor :type Actor%20Object%20Reference) (OtherComp :type Primitive%20Component%20Object%20Reference) (OtherBodyIndex :type Integer) (bFromSweep :type Boolean) (SweepResult :type Hit%20Result%20Structure%20%28by%20ref%29))
  ;[1 1 1] Grab and kill players
  (bind _asingredient_base_character (Utilities|Casting|CastToIngredientBaseCharacter OtherActor))
  (Variables|Default|SetIngredientInSphere _asingredient_base_character))

(event Custom|AttemptGrab
  (bind _ingredientinsphere (Variables|Default|GetIngredientInSphere))
  ;[1 1 1] Grab and kill players
  (if (Variables|Default|GetTryingGrab)
    (Utilities|IsValid _ingredientinsphere
      (:Is%20Valid
        (Class|IngredientBaseCharacter|KillThisIngredient _ingredientinsphere)
        (Transformation|AttachComponentToComponent _ingredientinsphere (Variables|Character|GetMesh) (Utilities|Name|MakeLiteralName "RightHandIndex3") "SnapToTarget" "SnapToTarget" "KeepWorld" true)
        (Variables|Default|SetTryingGrab false)
        (bind _output_get (Variables|Default|SetHoldingIngredient true))
        (AI|Components|Blackboard|SetValueasBool (AI|GetBlackboard 0) (Utilities|Name|MakeLiteralName "HoldingIngredient") _output_get)))))

(event Custom|ThrowOutIngredient
  ;[1 1 1] Grab and kill players
  (if (Variables|Default|GetHoldingIngredient)
    (Utilities|IsValid (Variables|Default|GetIngredientInSphere)
      (:Is%20Valid
        (Transformation|DetachFromComponent (Variables|/Script/Engine.Actor|GetRootComponent (Variables|Default|GetIngredientInSphere)) "KeepRelative" "KeepRelative" "KeepRelative" true)
        (Variables|Default|SetIngredientInSphere 0)
        (Variables|Default|SetHoldingIngredient false)))))

(event EventBeginPlay)

(event Collision|EventActorBeginOverlap
  (params (OtherActor :type Actor%20Object%20Reference)))

(fn ConstructionScript)