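; Game mode for the escape game that keeps registries of the characters and death zones added to it.
; AutoReposessCharacter makes player controller 0 possess the first registered character that is not dead.
; GetClosestDeathZone linearly scans the registered zones for the one nearest a given position.
; Despite the "AddToGameState" naming, both lists live on this game mode, and its event graph is empty.
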(event EventBeginPlay)

(event EventTick
  (params (DeltaSeconds :type Float%20%28single-precision%29)))

(fn ConstructionScript)

(fn AddCharactertoGameState
  (params (Character :type Ingredient%20Base%20Character%20Object%20Reference))
  (Utilities|Array|Add (Variables|Default|GetCharacters) Character))

(fn AutoReposessCharacter
  (for _array_element (Variables|Default|GetCharacters)
    (if (not (Variables|/Script/EscapeThePlate.IngredientBaseCharacter|GetbIsDead _array_element))
      (Pawn|Possess (Game|GetPlayerController 0) _array_element)
      (return))))

(fn AddDeathZonetoGameState
  (params (DeathZone :type Ingredient%20Death%20Zone%20Object%20Reference))
  (Utilities|Array|Add (Variables|Default|GetDeathZones) DeathZone))

(fn GetClosestDeathZone
  (params (Actor%20Position :type Vector))
  (bind _deathzones (Variables|Default|GetDeathZones))
  (if (== (Utilities|Array|Length _deathzones) 0)
    (return 0)
    (else
      (LocalVariables|SetClosestZone (Utilities|Array|Get(acopy) _deathzones))
      (for _array_element _deathzones
        (if (> (Math|Vector|VectorLength (- (Transformation|GetActorLocation (LocalVariables|GetClosestZone)) Actor%20Position)) (Math|Vector|VectorLength (- (Transformation|GetActorLocation _array_element) Actor%20Position)))
          (LocalVariables|SetClosestZone _array_element)))
      (return (LocalVariables|GetClosestZone)))))