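; Octopus character Blueprint that lets the octopus pick up and drop Grabbable actors.
; GrabObject releases any held item just ahead of the character with physics restored, or otherwise opens a half-second grab window.
; A GrabSphere begin-overlap during that window attaches the item to mesh socket Bone_010 with physics and collision off.
; JumpShrooms cannot bounce while held, and grabs and drops play AbilitySound.
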(event OnComponentBeginOverlap(GrabSphere)
  (params (OverlappedComponent :type Primitive%20Component%20Object%20Reference) (OtherActor :type Actor%20Object%20Reference) (OtherComp :type Primitive%20Component%20Object%20Reference) (OtherBodyIndex :type Integer) (bFromSweep :type Boolean) (SweepResult :type Hit%20Result%20Structure%20%28by%20ref%29))
  (bind _abilitysound (Variables|Default|GetAbilitySound))
  (if (and (Variables|Default|GetTryingGrab) (== (Variables|Default|GetGrabbedObject) 0))
    (bind _asgrabbable (Utilities|Casting|CastToGrabbable OtherActor))
    (bind _output_get (Variables|Default|SetGrabbedObject _asgrabbable))
    (if (not (Utilities|ClassIsChildOf (Utilities|GetClass _asgrabbable) "/Game/Blueprints/Interactables/JumpShroom.JumpShroom_C"))
      _
      (else
        (bind _asjump_shroom (Utilities|Casting|CastToJumpShroom _asgrabbable))
        (Variables|/Game/Blueprints/Interactables/JumpShroom.JumpShroom_C|SetCanBounce _asjump_shroom false)))
    (Physics|SetSimulatePhysics (Variables|/Game/Blueprints/Interactables/Grabbable.Grabbable_C|GetStaticMesh _output_get) false)
    (Collision|SetCollisionEnabled (Variables|/Game/Blueprints/Interactables/Grabbable.Grabbable_C|GetStaticMesh _output_get) "NoCollision")
    (Transformation|AttachComponentToComponent _asgrabbable (Variables|Character|GetMesh) "Bone_010" "SnapToTarget" "KeepWorld" "KeepWorld" false)
    (Utilities|IsValid _abilitysound
      (:Is%20Valid
        (Audio|PlaySound2D _abilitysound 1.0 1.0 0.0 0 0)))))

(event EventBeginPlay)

(event Collision|EventActorBeginOverlap
  (params (OtherActor :type Actor%20Object%20Reference)))

(event EventTick
  (params (DeltaSeconds :type Float%20%28single-precision%29)))

(event EventGrabObject
  (bind _abilitysound (Variables|Default|GetAbilitySound))
  (Utilities|IsValid (Variables|Default|GetGrabbedObject)
    (:Is%20Valid
      (Transformation|DetachFromActor (Variables|Default|GetGrabbedObject) "KeepWorld" "KeepWorld" "KeepWorld")
      (Transformation|SetActorLocation (Variables|Default|GetGrabbedObject) (+ (Transformation|GetActorLocation (Variables|Default|GetGrabbedObject)) (* (Math|Vector|GetForwardVector (Transformation|GetActorRotation)) 75)) false false)
      (Physics|SetSimulatePhysics (Variables|/Game/Blueprints/Interactables/Grabbable.Grabbable_C|GetStaticMesh (Variables|Default|GetGrabbedObject)) true)
      (Collision|SetCollisionEnabled (Variables|/Game/Blueprints/Interactables/Grabbable.Grabbable_C|GetStaticMesh (Variables|Default|GetGrabbedObject)) "QueryAndPhysics")
      (if (not (Utilities|ClassIsChildOf (Utilities|GetClass (Variables|Default|GetGrabbedObject)) "/Game/Blueprints/Interactables/JumpShroom.JumpShroom_C"))
        _
        (else
          (bind _asjump_shroom (Utilities|Casting|CastToJumpShroom (Variables|Default|GetGrabbedObject)))
          (Variables|/Game/Blueprints/Interactables/JumpShroom.JumpShroom_C|SetCanBounce _asjump_shroom true)))
      (Variables|Default|SetGrabbedObject 0)
      (Utilities|IsValid _abilitysound
        (:Is%20Valid
          (Audio|PlaySound2D _abilitysound 1.0 1.0 0.0 0 0))))
    (:Is%20Not%20Valid
      (Variables|Default|SetTryingGrab true)
      (Utilities|FlowControl|Delay 0.5)
      (Variables|Default|SetTryingGrab false))))

(fn ConstructionScript)