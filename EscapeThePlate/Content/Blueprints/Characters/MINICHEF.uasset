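; MINICHEF is a mini chef character Blueprint whose ability grabs and removes ingredient characters.
; GrabObject halts movement and opens a one-second grab window before restoring speed.
; During that window, sphere overlaps destroy other IngredientBaseCharacter actors and increment a counter, playing the ability sound until the count reaches the threshold that calls SaveThisIngredient.
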(event OnComponentBeginOverlap(Sphere)
  (params (OverlappedComponent :type Primitive%20Component%20Object%20Reference) (OtherActor :type Actor%20Object%20Reference) (OtherComp :type Primitive%20Component%20Object%20Reference) (OtherBodyIndex :type Integer) (bFromSweep :type Boolean) (SweepResult :type Hit%20Result%20Structure%20%28by%20ref%29))
  (bind _abilitysound (Variables|Default|GetAbilitySound))
  (if (and (!= OtherActor self) (Variables|Default|GetTryingGrab))
    (bind _asingredient_base_character (Utilities|Casting|CastToIngredientBaseCharacter OtherActor))
    (Actor|DestroyActor _asingredient_base_character)
    (bind _output_get (Variables|Default|SetGrabbed%20Count (+ (Variables|Default|GetGrabbed%20Count) 1)))
    (if (>= _output_get 6)
      (Class|IngredientBaseCharacter|SaveThisIngredient)
      (else
        (Utilities|IsValid _abilitysound
          (:Is%20Valid
            (Audio|PlaySound2D _abilitysound 1.0 1.0 0.0 0 0)))))))

(event EventBeginPlay)

(event Collision|EventActorBeginOverlap
  (params (OtherActor :type Actor%20Object%20Reference)))

(event EventTick
  (params (DeltaSeconds :type Float%20%28single-precision%29)))

(event EventGrabObject
  (Variables|Default|SetMoveSpeed 0.0)
  (Variables|Default|SetTryingGrab true)
  (Utilities|FlowControl|Delay 1.0)
  (Variables|Default|SetTryingGrab false)
  (Variables|Default|SetMoveSpeed 0.5))

(fn ConstructionScript)