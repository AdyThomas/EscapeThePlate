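; AI human character that spots usable ingredient characters, grabs and kills them, and can throw them out.
; A looping timer box-traces ahead, skips sneaking salmon, confirms line of sight, then writes the detected target to the Blackboard.
; During a timed grab window, sphere overlap kills the ingredient and attaches it to the hand, pausing detection until thrown out.
; AI Perception sight logic remains but is disconnected.
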(event OnTargetPerceptionUpdated(AIPerception)
  (params (Actor :type Actor%20Object%20Reference) (Stimulus :type AI%20Stimulus%20Structure))
  ;[1 1 1] Vision detection for ingredient
)

(event OnComponentBeginOverlap(GrabSphere)
  (params (OverlappedComponent :type Primitive%20Component%20Object%20Reference) (OtherActor :type Actor%20Object%20Reference) (OtherComp :type Primitive%20Component%20Object%20Reference) (OtherBodyIndex :type Integer) (bFromSweep :type Boolean) (SweepResult :type Hit%20Result%20Structure%20%28by%20ref%29))
  ;[1 1 1] Grab and kill players
  (if (Variables|Default|GetTryingGrab)
    (bind _asingredient_base_character (Utilities|Casting|CastToIngredientBaseCharacter OtherActor))
    (Class|IngredientBaseCharacter|KillThisIngredient _asingredient_base_character)
    (Collision|SetCollisionEnabled (Variables|/Script/Engine.Character|GetCapsuleComponent _asingredient_base_character) "NoCollision")
    (Transformation|AttachComponentToComponent _asingredient_base_character (Variables|Character|GetMesh) "RightHandIndex3" "SnapToTarget" "KeepRelative" "KeepWorld" false)
    (Variables|Default|SetHeldIngredient _asingredient_base_character)
    (bind _output_get (Variables|Default|SetHoldingIngredient true))
    (AI|Components|Blackboard|SetValueasBool (AI|GetBlackboard 0) (Utilities|Name|MakeLiteralName "HoldingIngredient") _output_get)))

(event Custom|AttemptGrab
  ;[1 1 1] Grab and kill players
  (Variables|Default|SetTryingGrab true)
  (Utilities|FlowControl|Delay 0.7)
  (Variables|Default|SetTryingGrab false))

(event Custom|ThrowOutIngredient
  ;[1 1 1] Grab and kill players
  (if (Variables|Default|GetHoldingIngredient)
    (Variables|Default|SetDetectedIngredient 0)
    (Transformation|DetachFromActor (Variables|Default|GetHeldIngredient) "KeepWorld" "KeepWorld" "KeepWorld")
    (Rendering|SetVisibility (Variables|/Script/Engine.Character|GetCapsuleComponent (Variables|Default|GetHeldIngredient)) false true)
    (Variables|Default|SetHeldIngredient 0)
    (Variables|Default|SetHoldingIngredient false)
    (Audio|PlaySoundatLocation "/Game/Assets/Sound/ThrowOutSC.ThrowOutSC" (Transformation|GetActorLocation) "0, 0, 0" 1.0 1.0 0.0 0 0 0)))

(event Custom|TraceForIngredient
  (bind _returnvalue (AI|GetBlackboard 0))
  (bind _returnvalue_2 (Transformation|GetActorLocation))
  (bind _returnvalue_3 (Transformation|GetActorRotation))
  (bind _returnvalue_4 (AI|GetBlackboard 0))
  (bind _returnvalue_5 (AI|GetBlackboard 0))
  (bind _returnvalue_6 (Math|Vector|GetForwardVector _returnvalue_3))
  ;[1 1 1] Vision detection for ingredient
  (if (not (Variables|Default|GetHoldingIngredient))
    (Variables|Default|SetDetectedIngredient 0)
    (bind (_outhits _returnvalue_7) (Class|KismetSystemLibrary|BoxTraceMultiforObjects (+ _returnvalue_2 (* _returnvalue_6 100)) (+ _returnvalue_2 (* _returnvalue_6 120)) "250.000000,200.000000,100.000000" "0, 0, 0" (Variables|Default|GetTraceType) false 0 "ForDuration" true))
    (if _returnvalue_7
      (bind _array_element (Utilities|Array|ForEachLoopwithBreak _outhits :!label _label)
        (:LoopBody
          (if (Utilities|ClassIsChildOf (Utilities|GetClass (.HitActor (Collision|BreakHitResult _array_element))) "/Script/EscapeThePlate.IngredientBaseCharacter")
            (if (Utilities|ClassIsChildOf (Utilities|GetClass (.HitActor (Collision|BreakHitResult _array_element))) "/Script/EscapeThePlate.SalmonCharacter")
              (bind _assalmon_character (Utilities|Casting|CastToSalmonCharacter (.HitActor (Collision|BreakHitResult _array_element))))
              (if (not (Variables|/Script/EscapeThePlate.SalmonCharacter|GetbIsSneaking _assalmon_character))
                (bind _returnvalue_8 (Class|IngredientBaseCharacter|IsIngredientUsable _assalmon_character))
                (if _returnvalue_8
                  (Variables|Default|SetDetectedIngredient _assalmon_character)
                  (goto _label Break)))
              (else
                (bind _asingredient_base_character (Utilities|Casting|CastToIngredientBaseCharacter (.HitActor (Collision|BreakHitResult _array_element))))
                (bind _returnvalue_9 (Class|IngredientBaseCharacter|IsIngredientUsable _asingredient_base_character))
                (if _returnvalue_9
                  (Variables|Default|SetDetectedIngredient _asingredient_base_character)
                  (goto _label Break))))))
        (:Completed
          (Utilities|IsValid (Variables|Default|GetDetectedIngredient)
            (:Is%20Valid
              (bind (_outhit _returnvalue_10) (Collision|LineTraceByChannel (Transformation|GetActorLocation) (Transformation|GetActorLocation (Variables|Default|GetDetectedIngredient)) "TraceTypeQuery1" false 0 "ForOneFrame"))
              (if _returnvalue_10
                (if (== (.HitActor (Collision|BreakHitResult _outhit)) (Variables|Default|GetDetectedIngredient))
                  (AI|Components|Blackboard|SetValueasBool _returnvalue_5 (Utilities|Name|MakeLiteralName "IngredientSeen") true :!label _label_2)
                  (AI|Components|Blackboard|SetValueasObject _returnvalue_5 (Utilities|Name|MakeLiteralName "DetectedCharacter") (Variables|Default|GetDetectedIngredient))
                  (else
                    (Variables|Default|SetDetectedIngredient 0)
                    (AI|Components|Blackboard|SetValueasBool _returnvalue (Utilities|Name|MakeLiteralName "IngredientSeen") false)
                    (AI|Components|Blackboard|SetValueasObject _returnvalue (Utilities|Name|MakeLiteralName "DetectedCharacter") 0)))
                (else
                  (goto _label_2))))
            (:Is%20Not%20Valid
              (AI|Components|Blackboard|SetValueasBool _returnvalue_4 (Utilities|Name|MakeLiteralName "IngredientSeen") false :!label _label_3)
              (AI|Components|Blackboard|SetValueasObject _returnvalue_4 (Utilities|Name|MakeLiteralName "DetectedCharacter") 0)))))
      (else
        (goto _label_3)))))

(event EventBeginPlay
  ;[1 1 1] Vision detection for ingredient
  (Utilities|Time|SetTimerbyEvent (delegate Custom|TraceForIngredient) 0.25 true))

(fn ConstructionScript)

(fn GetStatus
  (bind _returnvalue (AI|GetBlackboard 0))
  (Utilities|IsValid _returnvalue
    (:Is%20Valid
      (return (Class|BlackboardComponent|GetValueasEnum _returnvalue (Utilities|Name|MakeLiteralName "HumanStatus"))))
    (:Is%20Not%20Valid
      (return 0))))